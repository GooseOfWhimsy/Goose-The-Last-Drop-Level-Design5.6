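; BP_FlashingLight is an alarm light actor that pulses its Alarm light component between dark and full brightness from BeginPlay.
; Two timelines alternate: LightFlash lerps the intensity up, then Timeline lerps it back down.
; The cycle restarts only while LightFlashing is false, inverting what the variable's name suggests.
; Tick prints LightFlash's intensity every frame as debug output.
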(event `self.ReceiveBeginPlay`
  (bind (_direction _intensity) (`Timeline|LightFlash` :!label _label)
    (:`Update`
      (set `self.Light Lerp` _intensity)
      (`LightComponent.SetIntensity` (`self.Alarm`) (`KismetMathLibrary.Lerp` 0.0 10000.0 (`self.Light Lerp`))))
    (:`Finished`
      (bind (_direction_2 _intensity_2) (`Timeline|Timeline` :!via `PlayFromStart`)
        (:`Update`
          (set `self.Light Lerp` _intensity_2)
          (`LightComponent.SetIntensity` (`self.Alarm`) (`KismetMathLibrary.Lerp` 10000.0 0.0 (`self.Light Lerp`))))
        (:`Finished`
          (if (not (`self.LightFlashing`))
            (goto _label :!via `PlayFromStart`)))))))

(event `self.ReceiveTick`
  (params (DeltaSeconds :type "Float (single-precision)"))
  (`KismetSystemLibrary.PrintString` (`KismetStringLibrary.Conv_DoubleToString` (stale `self.ReceiveBeginPlay` _intensity))))

(fn `UserConstructionScript`)