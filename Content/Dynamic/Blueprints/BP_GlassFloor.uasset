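; BP_GlassFloor is a glass floor that shakes under a BP_BodyChar and breaks when a frozen bubble drops onto it.
; A second collider briefly arms BubbleDrop when a BP_FrozenBubble passes, letting a "Heavy"-tagged bubble on the main collider destroy the actor after a short delay.
; For characters, a timeline jitters the floor mesh, restores its once-saved location on finish, then re-enters the bubble check.
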(event `self.ReceiveTick`
  (params (DeltaSeconds :type "Float (single-precision)")))

(event `self.Collider.OnComponentBeginOverlap`
  (params (OverlappedComponent :type "PrimitiveComponent Object Reference") (OtherActor :type "Actor Object Reference") (OtherComp :type "PrimitiveComponent Object Reference") (OtherBodyIndex :type Integer) (bFromSweep :type Boolean) (SweepResult :type "HitResult Structure (by ref)"))
  (bind _floor (`self.Floor`))
  (bind _bubbledrop_ (`self.BubbleDrop?`))
  (if (`self.ActorHasTag` OtherActor "Heavy")
    (cast `/Game/Dynamic/Blueprints/Characters/BubbleChar/BP_FrozenBubble` OtherActor :!label _label)
    (`KismetSystemLibrary.PrintString` (`KismetStringLibrary.Conv_BoolToString` _bubbledrop_))
    (if _bubbledrop_
      (`KismetSystemLibrary.Delay` 0.5)
      (`self.K2_DestroyActor`))
    (else
      (cast `/Game/Dynamic/Blueprints/Characters/BodyChar/BP_BodyChar` OtherActor)
      (`|ExecutionSequence`
        (:`then_0`
          (`/Engine/EditorBlueprintResources/StandardMacros.DoOnce` false
            (:`Completed`
              (set `self.Start location` (`SceneComponent.K2_GetComponentLocation` (`self.Floor`))))))
        (:`then_1`
          (bind (_direction _shake_vector) (`Timeline|Shake` :!via `PlayFromStart` :!label _label_2)
            (:`Update`
              (`SceneComponent.K2_AddRelativeLocation` _floor (`KismetMathLibrary.MakeVector` (.x _shake_vector) 0.0 (* (.x _shake_vector) 0.25)) false false))
            (:`Finished`
              (`SceneComponent.K2_SetWorldLocation` _floor (`self.Start location`) false false)
              (goto _label))))))))

(event `self.Collider.OnComponentEndOverlap`
  (params (OverlappedComponent :type "PrimitiveComponent Object Reference") (OtherActor :type "Actor Object Reference") (OtherComp :type "PrimitiveComponent Object Reference") (OtherBodyIndex :type Integer))
  (cast `/Game/Dynamic/Blueprints/Characters/BodyChar/BP_BodyChar` OtherActor)
  (goto _label_2 :!via `Stop`))

(event `self.Collider1.OnComponentBeginOverlap`
  (params (OverlappedComponent :type "PrimitiveComponent Object Reference") (OtherActor :type "Actor Object Reference") (OtherComp :type "PrimitiveComponent Object Reference") (OtherBodyIndex :type Integer) (bFromSweep :type Boolean) (SweepResult :type "HitResult Structure (by ref)"))
  (cast `/Game/Dynamic/Blueprints/Characters/BubbleChar/BP_FrozenBubble` OtherActor)
  (set `self.BubbleDrop?` true)
  (`KismetSystemLibrary.Delay` 2.0)
  (set `self.BubbleDrop?` false))

(fn `UserConstructionScript`)