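; BP_playerkillzonechase is a moving kill zone that restarts the level when it catches the player character.
; The Startchase event plays the Chase timeline, which lerps the actor between two hardcoded world positions.
; Overlapping its Box with BP_BodyChar fades the camera and audio out, then runs the RestartLevel console command after a delay.
; An unconnected node would instead teleport the character to the Billboard's location.
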(event `self.Box.OnComponentBeginOverlap`
  (params (OverlappedComponent :type "PrimitiveComponent Object Reference") (OtherActor :type "Actor Object Reference") (OtherComp :type "PrimitiveComponent Object Reference") (OtherBodyIndex :type Integer) (bFromSweep :type Boolean) (SweepResult :type "HitResult Structure (by ref)"))
  (bind _asbp_body_char (cast `/Game/Dynamic/Blueprints/Characters/BodyChar/BP_BodyChar` OtherActor))
  (`PlayerCameraManager.StartCameraFade` :`self` (`GameplayStatics.GetPlayerCameraManager` 0) :`ToAlpha` 1.0 :`Duration` 0.5 :`bShouldFadeAudio` true :`bHoldWhenFinished` true)
  (`KismetSystemLibrary.Delay` 1.5)
  (`KismetSystemLibrary.ExecuteConsoleCommand` "RestartLevel" null))

(event `Start chase`
  (bind (_direction _chase) (`Timeline|Chase`)
    (:`Update`
      (`self.K2_SetActorLocation` (`KismetMathLibrary.VLerp` (1000.0 -400.0 4790.0) (1990.0 4850.0 4790.0) _chase)))))

(fn `UserConstructionScript`)