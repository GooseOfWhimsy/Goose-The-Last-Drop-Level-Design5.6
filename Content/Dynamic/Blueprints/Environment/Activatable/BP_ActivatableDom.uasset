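; Activatable environment actor with three components, Dom1 to Dom3, that snap back to their starting poses when activated or deactivated.
; BeginPlay caches each world transform, which Activate/Deactivate restores by teleport.
; Only Dom3 has physics simulation switched off for the teleport and back on afterwards.
; The separate Reset event ignores the cached transforms and teleports only Dom3 to the world origin.
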(event `self.ReceiveBeginPlay`
  (set `self.Reset Trans 1` (`SceneComponent.K2_GetComponentToWorld` (`self.Dom 1`)))
  (set `self.Reset Trans 2` (`SceneComponent.K2_GetComponentToWorld` (`self.Dom 2`)))
  (set `self.Reset Trans 3` (`SceneComponent.K2_GetComponentToWorld` (`self.Dom 3`))))

(event `self.Activate/Deactivate`
  (bind (_reset_trans_1_location _reset_trans_1_rotation) (`KismetMathLibrary.BreakTransform` (`self.Reset Trans 1`)))
  (bind _dom_3 (`self.Dom 3`))
  (bind (_reset_trans_2_location _reset_trans_2_rotation) (`KismetMathLibrary.BreakTransform` (`self.Reset Trans 2`)))
  (bind (_reset_trans_3_location _reset_trans_3_rotation) (`KismetMathLibrary.BreakTransform` (`self.Reset Trans 3`)))
  (`SceneComponent.K2_SetWorldLocationAndRotation` (`self.Dom 1`) _reset_trans_1_location _reset_trans_1_rotation false true)
  (`SceneComponent.K2_SetWorldLocationAndRotation` (`self.Dom 2`) _reset_trans_2_location _reset_trans_2_rotation false true)
  (`PrimitiveComponent.SetSimulatePhysics` _dom_3 false)
  (`SceneComponent.K2_SetWorldLocationAndRotation` _dom_3 _reset_trans_3_location _reset_trans_3_rotation false true)
  (`PrimitiveComponent.SetSimulatePhysics` _dom_3 true))

(event `Reset`
  (`SceneComponent.K2_SetWorldLocation` (`self.Dom 3`) (0.0 0.0 0.0) false true))

(fn `UserConstructionScript`
  (`parent.UserConstructionScript`))