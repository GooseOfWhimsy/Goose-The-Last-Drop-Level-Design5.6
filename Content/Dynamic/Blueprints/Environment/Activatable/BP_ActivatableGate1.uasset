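; Activatable gate Blueprint that toggles its position each time its Activate/Deactivate event fires.
; BeginPlay stores the starting location, then a FlipFlop alternates the gate instantly between the world origin and that stored location, without sweep.
; A box overlap casts the entering actor to BP_ActivatableDom and calls Reset on it.
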(event `self.ReceiveBeginPlay`
  (set `self.Start Loc` (`self.K2_GetActorLocation`)))

(event `self.Activate/Deactivate`
  (`/Engine/EditorBlueprintResources/StandardMacros.FlipFlop`
    (:`A`
      (`self.K2_SetActorLocation` (0.0 0.0 0.0)))
    (:`B`
      (`self.K2_SetActorLocation` (`self.Start Loc`)))))

(event `self.Box.OnComponentBeginOverlap`
  (params (OverlappedComponent :type "PrimitiveComponent Object Reference") (OtherActor :type "Actor Object Reference") (OtherComp :type "PrimitiveComponent Object Reference") (OtherBodyIndex :type Integer) (bFromSweep :type Boolean) (SweepResult :type "HitResult Structure (by ref)"))
  (bind _asbp_activatable_dom (cast `/Game/Dynamic/Blueprints/Environment/Activatable/BP_ActivatableDom` OtherActor))
  (`/Game/Dynamic/Blueprints/Environment/Activatable/BP_ActivatableDom.Reset` _asbp_activatable_dom))

(fn `UserConstructionScript`
  (`parent.UserConstructionScript`))