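; Activatable door made of two cube meshes that toggles between open and closed on each Activate/Deactivate event.
; BeginPlay caches each cube's relative X, then a FlipFlop switches DoorAlpha to lerp both cubes between that start and a shared fixed X.
; The move is an instant snap with no timeline, and the DoOnce resets in the same Sequence, so every event toggles it.
; A debug "Door open" string prints on either toggle.
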(event `self.ReceiveBeginPlay`
  (bind _relativelocation_x (`KismetMathLibrary.BreakVector` (`SceneComponent.RelativeLocation` (`self.Cube`))))
  (bind _relativelocation_x_2 (`KismetMathLibrary.BreakVector` (`SceneComponent.RelativeLocation` (`self.Cube1`))))
  (set `self.Starting Location Cube 1` _relativelocation_x_2)
  (set `self.Starting Location Cube` _relativelocation_x))

(event `self.Activate/Deactivate`
  (bind (_relative_location_cube_1_x _relative_location_cube_1_y _relative_location_cube_1_z) (`KismetMathLibrary.BreakVector` (`self.Relative Location Cube 1`)))
  (bind (_relative_location_cube_x _relative_location_cube_y _relative_location_cube_z) (`KismetMathLibrary.BreakVector` (`self.Relative Location Cube`)))
  (`|ExecutionSequence`
    (:`then_0`
      (set `self.Relative Location Cube 1` (`SceneComponent.RelativeLocation` (`self.Cube1`)))
      (set `self.Relative Location Cube` (`SceneComponent.RelativeLocation` (`self.Cube`)))
      (`/Engine/EditorBlueprintResources/StandardMacros.DoOnce` false :!label _label
        (:`Completed`
          (`/Engine/EditorBlueprintResources/StandardMacros.FlipFlop`
            (:`A`
              (set `self.Door Alpha` 1.0))
            (:`B`
              (set `self.Door Alpha` 0.0)))
          (`SceneComponent.K2_SetRelativeLocation` (`self.Cube1`) (`KismetMathLibrary.MakeVector` (`KismetMathLibrary.Lerp` (`self.Starting Location Cube 1`) 100.0 (`self.Door Alpha`)) _relative_location_cube_1_y _relative_location_cube_1_z) false false)
          (`SceneComponent.K2_SetRelativeLocation` (`self.Cube`) (`KismetMathLibrary.MakeVector` (`KismetMathLibrary.Lerp` (`self.Starting Location Cube`) 100.0 (`self.Door Alpha`)) _relative_location_cube_y _relative_location_cube_z) false false)
          (`KismetSystemLibrary.PrintString` "Door open"))))
    (:`then_1`
      (goto _label :!via `Reset`))))

(fn `UserConstructionScript`
  (`parent.UserConstructionScript`))