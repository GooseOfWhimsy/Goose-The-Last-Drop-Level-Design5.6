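; Environmental cold fan that turns the player's bubble into a frozen bubble when it lingers in the fan's collision.
; Overlap events toggle a freezing flag, and Tick runs a three-second Delay before rechecking it.
; It then destroys any frozen bubble flagged on BP_BodyChar and, behind a DoOnce reset on exit, spawns BP_FrozenBubble at BP_BubbleChar's location and pops the original.
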(event `self.ReceiveTick`
  (params (DeltaSeconds :type "Float (single-precision)"))
  (if (`self.IsFreezing?`)
    (`KismetSystemLibrary.PrintString` "Timer started!")
    (`KismetSystemLibrary.Delay` 3.0)
    (if (`self.IsFreezing?`)
      (bind _returnvalue (`GameplayStatics.GetActorOfClass` "/Game/Dynamic/Blueprints/Characters/BodyChar/BP_BodyChar.BP_BodyChar_C"))
      (if (`/Game/Dynamic/Blueprints/Characters/BodyChar/BP_BodyChar.FrozenSpawned?` _returnvalue)
        (bind _returnvalue_2 (`GameplayStatics.GetActorOfClass` "/Game/Dynamic/Blueprints/Characters/BubbleChar/BP_FrozenBubble.BP_FrozenBubble_C"))
        (`self.K2_DestroyActor` _returnvalue_2)
        (set `/Game/Dynamic/Blueprints/Characters/BodyChar/BP_BodyChar.FrozenSpawned?` false _returnvalue))
      (bind _returnvalue_3 (`GameplayStatics.GetActorOfClass` "/Game/Dynamic/Blueprints/Characters/BubbleChar/BP_BubbleChar.BP_BubbleChar_C"))
      (`/Engine/EditorBlueprintResources/StandardMacros.DoOnce` false :!label _label
        (:`Completed`
          (`|SpawnActorFromClass` "/Game/Dynamic/Blueprints/Characters/BubbleChar/BP_FrozenBubble.BP_FrozenBubble_C" (`KismetMathLibrary.MakeTransform` (`self.K2_GetActorLocation` _returnvalue_3)) "Undefined" "MultiplyWithRoot" null null)
          (bind _returnvalue_4 (`GameplayStatics.GetActorOfClass` "/Game/Dynamic/Blueprints/Characters/BodyChar/BP_BodyChar.BP_BodyChar_C"))
          (set `/Game/Dynamic/Blueprints/Characters/BodyChar/BP_BodyChar.FrozenSpawned?` true _returnvalue_4)
          (bind _returnvalue_5 (`GameplayStatics.GetActorOfClass` "/Game/Dynamic/Blueprints/Characters/BubbleChar/BP_BubbleChar.BP_BubbleChar_C"))
          (`/Game/Dynamic/Blueprints/Characters/BubbleChar/BP_BubbleChar.Pop` _returnvalue_5))))))

(event `self.Fan Collision.OnComponentBeginOverlap`
  (params (OverlappedComponent :type "PrimitiveComponent Object Reference") (OtherActor :type "Actor Object Reference") (OtherComp :type "PrimitiveComponent Object Reference") (OtherBodyIndex :type Integer) (bFromSweep :type Boolean) (SweepResult :type "HitResult Structure (by ref)"))
  (cast `/Game/Dynamic/Blueprints/Characters/BubbleChar/BP_BubbleChar` OtherActor)
  (set `self.IsFreezing?` true))

(event `self.Fan Collision.OnComponentEndOverlap`
  (params (OverlappedComponent :type "PrimitiveComponent Object Reference") (OtherActor :type "Actor Object Reference") (OtherComp :type "PrimitiveComponent Object Reference") (OtherBodyIndex :type Integer))
  (cast `/Game/Dynamic/Blueprints/Characters/BubbleChar/BP_BubbleChar` OtherActor)
  (set `self.IsFreezing?` false)
  (goto _label :!via `Reset`))

(fn `UserConstructionScript`)