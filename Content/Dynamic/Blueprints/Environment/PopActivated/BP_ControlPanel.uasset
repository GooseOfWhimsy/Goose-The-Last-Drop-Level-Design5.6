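; BP_ControlPanel is an environment control panel that is triggered once when a BP_FrozenBubble overlaps its Box.
; The overlap toggles BPActivatable, then after a short delay spawns sparks at the Billboard, swaps a mesh material and plays a 2D sound.
; The Box is destroyed after a second delay to stop further triggers.
; The pop interaction event is present but empty.
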(event `/Game/Dynamic/Blueprints/Core/BPI_PopInteract.BPI_PopInteract`)

(event `self.Box.OnComponentBeginOverlap`
  (params (OverlappedComponent :type "PrimitiveComponent Object Reference") (OtherActor :type "Actor Object Reference") (OtherComp :type "PrimitiveComponent Object Reference") (OtherBodyIndex :type Integer) (bFromSweep :type Boolean) (SweepResult :type "HitResult Structure (by ref)"))
  (cast `/Game/Dynamic/Blueprints/Characters/BubbleChar/BP_FrozenBubble` OtherActor)
  (`/Game/Dynamic/Blueprints/Environment/Activatable/BP_ActivatableParent.Activate/Deactivate` (`self.BP_Activatable`))
  (`KismetSystemLibrary.Delay` 0.3)
  (`NiagaraFunctionLibrary.SpawnSystemAtLocation` "/Game/Dynamic/Blueprints/Environment/NS_Sparks.NS_Sparks" (`SceneComponent.K2_GetComponentLocation` (`self.Billboard`)))
  (`PrimitiveComponent.SetMaterial` (`self.StaticMesh`) 1 "/Engine/EngineMaterials/BaseFlattenMaterial.BaseFlattenMaterial")
  (`GameplayStatics.PlaySound2D` "/Game/Dynamic/Audio/Events/MS_ControlPanel.MS_ControlPanel" 1.0 1.0 0.0 null null)
  (`KismetSystemLibrary.Delay` 0.2)
  (`ActorComponent.K2_DestroyComponent` (`self.Box`)))

(fn `UserConstructionScript`)